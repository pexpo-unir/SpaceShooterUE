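; Movement component for the space shooter that moves its owning actor every tick from Direction and Speed.
; MovementTick scales both by delta time, applies the result along the owner's right and forward vectors, and sets the new location directly.
; When a Background actor is valid, GetBackgroundBounds derives min and max from its actor bounds to clamp X and Y, leaving Z unclamped.
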(event EventTick
  (params (DeltaSeconds :type Float%20%28single-precision%29))
  (CallFunction|MovementTick DeltaSeconds))

(fn MovementTick
  (params (DeltaSeconds :type Float%20%28double-precision%29))
  (bind _returnvalue (Components|GetOwner))
  (bind _direction (Variables|Default|GetDirection))
  (bind _speed (Variables|Default|GetSpeed))
  (bind _returnvalue_2 (Transformation|GetActorRightVector _returnvalue))
  (bind _returnvalue_3 (Transformation|GetActorForwardVector _returnvalue))
  (bind _returnvalue_4 (Transformation|GetActorLocation _returnvalue))
  (bind _returnvalue_5 (* _direction _speed))
  (bind _returnvalue_6 (* DeltaSeconds _returnvalue_5))
  (bind _returnvalue_7 (* _returnvalue_2 _returnvalue_6))
  (bind _returnvalue_8 (* _returnvalue_6 _returnvalue_3))
  (bind _returnvalue_9 (+ _returnvalue_7 _returnvalue_8))
  (bind _returnvalue_10 (+ _returnvalue_4 _returnvalue_9))
  (Utilities|IsValid (Variables|Default|GetBackground)
    (:Is%20Valid
      (bind (_min _max) (CallFunction|GetBackgroundBounds))
      (Transformation|SetActorLocation _returnvalue (Math|Vector|MakeVector (Math|Float|Clamp(Float) (.x _returnvalue_10) (.x _min) (.x _max)) (Math|Float|Clamp(Float) (.y _returnvalue_10) (.y _min) (.y _max)) (.z _returnvalue_10)) false false))
    (:Is%20Not%20Valid
      (Transformation|SetActorLocation _returnvalue (Math|Vector|MakeVector (.x _returnvalue_10) (.y _returnvalue_10) (.z _returnvalue_10)) false false))))

(fn GetBackgroundBounds
  (bind _background (Variables|Default|GetBackground))
  (bind (_origin _boxextent) (Collision|GetActorBounds _background false false))
  (Utilities|IsValid _background
    (:Is%20Valid
      (return (- _origin _boxextent) (+ _origin _boxextent)))
    (:Is%20Not%20Valid
      (return "-99999.000000,-99999.000000,0.000000" "99999.000000,99999.000000,0.000000"))))