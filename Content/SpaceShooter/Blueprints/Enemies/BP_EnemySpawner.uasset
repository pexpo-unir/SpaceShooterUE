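; Enemy spawner for the space shooter that periodically spawns random ship classes from EnemyShips within its Box bounds.
; Tick counts down the spawn interval, which is re-sampled from SpawnFrequencyCurve using the game mode's GameProgress, so pacing follows progression.
; Each ship spawns at a random XY in the box at the spawner's Z, faces the left vector, and receives a BP_EnemyControllerBase AI controller.
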(event EventBeginPlay
  (Variables|Default|SetSpawnFrequencyCountdown (Variables|Default|GetSpawnFrequency))
  (bind _asbp_space_shooter_game_mode (Utilities|Casting|CastToBP_SpaceShooterGameMode (Game|GetGameMode)))
  (Variables|Default|SetAs%20BP%20Space%20Shooter%20Game%20Mode _asbp_space_shooter_game_mode))

(event EventTick
  (params (DeltaSeconds :type Float%20%28single-precision%29))
  (Variables|Default|SetSpawnFrequency (Math|Curves|GetFloatValue (Variables|Default|GetSpawnFrequencyCurve) (Math|Conversions|ToFloat(Integer) (Variables|/Game/SpaceShooter/Blueprints/BP_SpaceShooterGameMode.BP_SpaceShooterGameMode_C|GetGameProgress (Variables|Default|GetAs%20BP%20Space%20Shooter%20Game%20Mode)))))
  (bind _output_get (Variables|Default|SetSpawnFrequencyCountdown (- (Variables|Default|GetSpawnFrequencyCountdown) (* DeltaSeconds 1.0))))
  (if (<= _output_get 0.0)
    (CallFunction|SpawnRandomEnemy)
    (Variables|Default|SetSpawnFrequencyCountdown (Variables|Default|GetSpawnFrequency))))

(fn ConstructionScript)

(fn GetRandomShipEnemyClass
  (bind _enemyships (Variables|Default|GetEnemyShips))
  (return (Utilities|Array|Get(acopy) _enemyships (Math|Random|RandomIntegerinRange 0 (- (Utilities|Array|Length _enemyships) -1)))))

(fn SpawnRandomEnemy
  (bind _returnvalue (Transformation|GetActorLocation))
  (bind _box (Variables|Default|GetBox))
  (bind _returnvalue_2 (Components|Box|GetScaledBoxExtent _box))
  (bind _returnvalue_3 (Math|Random|RandomPointinBoundingBox _returnvalue _returnvalue_2))
  (bind _returnvalue_4 (Game|SpawnActorfromClass (CallFunction|GetRandomShipEnemyClass) (Math|Transform|MakeTransform (Math|Vector|MakeVector (.x _returnvalue_3) (.y _returnvalue_3) (.z (Transformation|GetActorLocation))) (Math|Conversions|RotationFromXVector (Class|KismetMathLibrary|VectorLeft)) "1.000000,1.000000,1.000000") "Undefined" "MultiplyWithRoot" 0 0))
  (Utilities|IsValid _returnvalue_4
    (:Is%20Valid
      (Variables|/Script/Engine.Pawn|SetAIControllerClass _returnvalue_4 "/Game/SpaceShooter/Blueprints/Enemies/BP_EnemyControllerBase.BP_EnemyControllerBase_C")
      (Pawn|SpawnDefaultController _returnvalue_4))))