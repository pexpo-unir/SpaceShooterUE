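; Base controller for Space Shooter enemies that drives a possessed BP_ShipPawn, tagged as Enemy, by simulating player input.
; A looping timer fires the ship's weapon, while Tick feeds SimulateMovementInput into its movement direction, which defaults to a constant right vector.
; On ship death it destroys the pawn, has a coin-flip chance to spawn a random power-up, increments game mode progress, then destroys itself.
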(event Custom|EventPressFire
  (bind _ship (Variables|Default|GetShip))
  ;[1 1 1] Fire simulation
  (Utilities|IsValid _ship
    (:Is%20Valid
      (Default|FireProjectile _ship))
    (:Is%20Not%20Valid
      (Utilities|Time|PauseTimerbyHandle (stale EventBeginPlay _returnvalue)))))

(event Custom|EventShipDead
  (bind _ship (Variables|Default|GetShip))
  ;[1 0 0] Dead
  (Variables|Default|SetPowerUpTransform (Transformation|GetActorLocation _ship))
  (Actor|DestroyActor _ship)
  ;[1 1 1] Spawn PowerUps (50% probability)
  (if (== (Math|Random|RandomIntegerinRange 0 1) 0)
    (Game|SpawnActorfromClass (Utilities|Array|Get(acopy) (Variables|Default|GetPowerUps) (Math|Random|RandomIntegerinRange 0 (- (Utilities|Array|Length (Variables|Default|GetPowerUps)) 1))) (Math|Transform|MakeTransform (Variables|Default|GetPowerUpTransform) "0, 0, 0" "1.000000,1.000000,1.000000") "Undefined" "MultiplyWithRoot" 0 0))
  ;[1 1 1] Increment Progress
  (bind _asbp_space_shooter_game_mode (Utilities|Casting|CastToBP_SpaceShooterGameMode (Game|GetGameMode)))
  (Default|IncrementProgress _asbp_space_shooter_game_mode 5)
  (Utilities|FlowControl|Delay 0.2)
  (Actor|DestroyActor))

(event EventBeginPlay
  ;[1 1 1] Fire simulation
  (bind _returnvalue (Utilities|Time|SetTimerbyEvent (delegate Custom|EventPressFire) (Variables|Default|GetFireRate) true)))

(event EventTick
  (params (DeltaSeconds :type Float%20%28single-precision%29))
  (bind _inputdirection (CallFunction|SimulateMovementInput))
  (Default|SetMovementDirection (Variables|Default|GetShip) (Math|Vector2D|Normalize2D (Math|Conversions|ToVector2D(Vector) _inputdirection))))

(event EventPossess
  (params (PossessedPawn :type Pawn%20Object%20Reference))
  (Utilities|FlowControl|Sequence
    (:then_0
      ;[1 1 1] Get Controlled Ship
      (bind _asbp_ship_pawn (Utilities|Casting|CastToBP_ShipPawn (Pawn|GetControlledPawn)))
      (Utilities|IsValid _asbp_ship_pawn
        (:Is%20Valid
          (bind _output_get (Variables|Default|SetShip _asbp_ship_pawn))
          (Utilities|Array|Add (Variables|/Script/Engine.Actor|GetTags _output_get) "Enemy")
          (Default|ChangeWeapon _output_get (Variables|/Game/SpaceShooter/Blueprints/Ships/BP_ShipPawn.BP_ShipPawn_C|GetWeapon _output_get)))))
    (:then_1
      ;[1 0 0] Dead
      (EventDispatchers|BindEventtoOnDeath (Variables|/Game/SpaceShooter/Blueprints/Ships/BP_ShipPawn.BP_ShipPawn_C|GetBP_DamageSystemComponent (Variables|Default|GetShip)) (delegate Custom|EventShipDead)))))

(fn ConstructionScript)

(fn SimulateMovementInput
  (return (Class|KismetMathLibrary|VectorRight)))