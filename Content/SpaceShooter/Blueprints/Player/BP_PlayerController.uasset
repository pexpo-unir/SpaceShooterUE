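; Player controller for the space shooter that drives the possessed BP_ShipPawn from Enhanced Input.
; On BeginPlay it adds the default mapping context, tags the ship as Player, passes it the background and equips the simple weapon.
; Move input becomes a normalized direction, zeroed on release, and shoot input fires projectiles.
; It binds the ship's damage, healing and death events to update HUD lives, signal death and show the cursor.
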(event Custom|EventShipTakeDamage
  (params (Amount :type Integer) (Lifes :type Integer))
  ;[1 1 1] Damage System
  (bind _asbp_hud (Utilities|Casting|CastToBP_HUD (HUD|GetHUD)))
  (Default|EventUpdateLifes _asbp_hud Lifes))

(event Custom|EventShipTakeHealing
  (params (Amount :type Integer) (Lifes :type Integer))
  ;[1 1 1] Damage System
  (bind _asbp_hud (Utilities|Casting|CastToBP_HUD (HUD|GetHUD)))
  (Default|EventUpdateLifes _asbp_hud Lifes))

(event Custom|EventShipDead
  ;[1 1 1] Damage System
  ;;[1 0 0] Comment
  (bind _asbp_hud (Utilities|Casting|CastToBP_HUD (HUD|GetHUD)))
  (Default|EventPlayerDead _asbp_hud)
  (Variables|Default|SetbShowMouseCursor true))

(event Input|EnhancedActionEvents|EnhancedInputActionIA_Move
  (params (ActionValue :type Vector%202D%20Structure) (ElapsedSeconds :type Float%20%28double-precision%29) (TriggeredSeconds :type Float%20%28double-precision%29) (InputAction :type Input%20Action%20Object%20Reference :default "/Game/SpaceShooter/Input/Actions/IA_Move.IA_Move"))
  ;[1 1 1] Movement
  (:Triggered
    (CallFunction|MoveShipPawn ActionValue :!label _label))
  (:Started
    (goto _label))
  (:Ongoing
    (goto _label))
  (:Canceled
    (CallFunction|MoveShipPawn :!label _label_2))
  (:Completed
    (goto _label_2)))

(event Input|EnhancedActionEvents|EnhancedInputActionIA_Shoot
  (params (ActionValue :type Boolean) (ElapsedSeconds :type Float%20%28double-precision%29) (TriggeredSeconds :type Float%20%28double-precision%29) (InputAction :type Input%20Action%20Object%20Reference :default "/Game/SpaceShooter/Input/Actions/IA_Shoot.IA_Shoot"))
  ;[1 1 1] Fire
  (:Triggered
    (CallFunction|FireProjectileShipPawn :!label _label))
  (:Started
    (goto _label))
  (:Ongoing
    (goto _label)))

(event EventBeginPlay
  (bind _returnvalue (PlayerController|LocalPlayerSubsystems|GetEnhancedInputLocalPlayerSubsystem))
  ;[1 1 1] Add Mapping Context
  (Utilities|IsValid _returnvalue
    (:Is%20Valid
      (Input|AddMappingContext _returnvalue "/Game/SpaceShooter/Input/IMC_SpaceShooterDefault.IMC_SpaceShooterDefault" 0 "(bIgnoreAllPressedKeysUntilRelease=True,bForceImmediately=False,bNotifyUserSettings=False)")
      (bind _asbp_ship_pawn (Utilities|Casting|CastToBP_ShipPawn (Pawn|GetControlledPawn)))
      (Utilities|IsValid _asbp_ship_pawn
        (:Is%20Valid
          (bind _output_get (Variables|Default|SetShip _asbp_ship_pawn))
          (Utilities|Array|Add (Variables|/Script/Engine.Actor|GetTags _output_get) "Player")
          (Variables|/Game/SpaceShooter/Blueprints/MovementComponent/BP_MovementComponent.BP_MovementComponent_C|SetBackground (Variables|/Game/SpaceShooter/Blueprints/Ships/BP_ShipPawn.BP_ShipPawn_C|GetBP_MovementComponent _output_get) (Variables|Default|GetBackground))
          (Default|ChangeWeapon _output_get "/Game/SpaceShooter/Blueprints/Weapons/BP_SimpleWeapon.BP_SimpleWeapon_C")
          ;[1 1 1] Damage System
          (EventDispatchers|BindEventtoOnTakeDamage (Variables|/Game/SpaceShooter/Blueprints/Ships/BP_ShipPawn.BP_ShipPawn_C|GetBP_DamageSystemComponent (Variables|Default|GetShip)) (delegate Custom|EventShipTakeDamage))
          (EventDispatchers|BindEventtoOnTakeHealing (Variables|/Game/SpaceShooter/Blueprints/Ships/BP_ShipPawn.BP_ShipPawn_C|GetBP_DamageSystemComponent (Variables|Default|GetShip)) (delegate Custom|EventShipTakeHealing))
          ;;[1 0 0] Comment
          (EventDispatchers|BindEventtoOnDeath (Variables|/Game/SpaceShooter/Blueprints/Ships/BP_ShipPawn.BP_ShipPawn_C|GetBP_DamageSystemComponent (Variables|Default|GetShip)) (delegate Custom|EventShipDead)))))
    (:Is%20Not%20Valid
      (Development|PrintText "Enhanced Input is not valid!" true true "(R=1.000000,G=0.000000,B=0.000000,A=1.000000)" 1e+01))))

(fn ConstructionScript)

(fn MoveShipPawn
  (params (InputDirection :type Vector%202D%20Structure))
  (Default|SetMovementDirection (Variables|Default|GetShip) (Math|Vector2D|Normalize2D InputDirection)))

(fn FireProjectileShipPawn
  (Default|FireProjectile (Variables|Default|GetShip)))