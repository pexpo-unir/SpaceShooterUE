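; BP_DamageSystemComponent is a component in the SpaceShooter game that tracks an owner's lives for damage and healing.
; On BeginPlay it fills Lifes to MaxLifes.
; TakeDamage and TakeHealing clamp Lifes between zero and MaxLifes and broadcast OnTakeDamage, which also serves as the healing notification.
; TakeDamage additionally fires OnDeath whenever Lifes reaches zero.
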(event EventBeginPlay
  (Variables|Default|SetLifes (Variables|Default|GetMaxLifes)))

(fn TakeDamage
  (params (Amount :type Integer))
  ;[1 1 1] Take Damage
  (bind _output_get (Variables|Default|SetLifes (Math|Integer|Clamp(Integer) (- (Variables|Default|GetLifes) Amount) 0 (Variables|Default|GetMaxLifes))))
  (Default|CallOnTakeDamage Amount _output_get)
  ;[1 1 1] If Lifes (1 <= 0) CallOn Death
  (if (<= _output_get 0)
    (Default|CallOnDeath)))

(fn TakeHealing
  (params (Amount :type Integer))
  (bind _output_get (Variables|Default|SetLifes (Math|Integer|Clamp(Integer) (+ Amount (Variables|Default|GetLifes)) 0 (Variables|Default|GetMaxLifes))))
  (Default|CallOnTakeDamage Amount _output_get))