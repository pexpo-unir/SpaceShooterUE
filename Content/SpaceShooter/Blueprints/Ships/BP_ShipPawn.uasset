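; Base ship pawn for a space shooter that moves, fires a swappable weapon and takes damage or healing.
; Movement input goes to a movement component, while damage and healing are forwarded to a damage system component.
; On possession it spawns its weapon on a socket and copies its first tag onto it, and firing delegates to that instance.
; Overlapping another ship that shares no tag deals one damage to itself.
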(event Custom|EventFireProjectileCooldownFinished
  (Variables|Default|SetCanFireProjectile true))

(event Collision|EventActorBeginOverlap
  (params (OtherActor :type Actor%20Object%20Reference))
  (Utilities|Casting|CastToBP_ShipPawn OtherActor)
  (bind _hasonetag (CallFunction|CheckifContainsatLeastOneTag self OtherActor))
  (if (not _hasonetag)
    (CallFunction|TakeDamage 1)))

(event EventPossessed
  (params (NewController :type Controller%20Object%20Reference))
  (CallFunction|ChangeWeapon (Variables|Default|GetWeapon)))

(event EventTakeHealing
  (params (Healing :type Integer))
  (Default|TakeHealing (Variables|Default|GetBP_DamageSystemComponent) Healing))

(event EventTakeDamage
  (params (Damage :type Integer))
  (Default|TakeDamage (Variables|Default|GetBP_DamageSystemComponent) Damage))

(fn ConstructionScript)

(fn SetMovementDirection
  (params (InputDirection :type Vector%202D%20Structure))
  (Variables|/Game/SpaceShooter/Blueprints/MovementComponent/BP_MovementComponent.BP_MovementComponent_C|SetDirection (Variables|Default|GetBP_MovementComponent) (Math|Conversions|ToVector(Vector2D) InputDirection)))

(fn FireProjectile
  (Default|Fire (Variables|Default|GetWeaponInstance)))

(fn ChangeWeapon
  (params (WeaponClass :type BP%20Weapon%20Base%20Class%20Reference))
  (Utilities|IsValid (Variables|Default|GetWeaponInstance)
    (:Is%20Valid
      (Actor|DestroyActor (Variables|Default|GetWeaponInstance)))
    (:Is%20Not%20Valid
      _))
  (bind _returnvalue (Game|SpawnActorfromClass WeaponClass (Transformation|GetRelativeTransform (Variables|Default|GetWeaponSocket)) "Undefined" "MultiplyWithRoot" 0 0))
  (Variables|Default|SetCanFireProjectile true)
  (bind _output_get (Variables|Default|SetWeaponInstance _returnvalue))
  (Utilities|Array|Add (Variables|/Script/Engine.Actor|GetTags _output_get) (Utilities|Array|Get(acopy) (Variables|Actor|GetTags)))
  (Transformation|AttachComponentToComponent _output_get (Variables|Default|GetWeaponSocket) "None" "KeepRelative" "KeepRelative" "KeepRelative" true))