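; Enemy ship pawn for the space shooter that adds a sideways drift to its inherited movement, producing an oblique path.
; On BeginPlay it picks a horizontal direction toward the center, positive X if spawned at negative X and negative X otherwise.
; Each tick, after the parent Tick, it offsets its X location along that direction, scaled by the movement component's Speed and delta time.
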(event EventBeginPlay
  (|CallParentFunction)
  (if (< (.x (Transformation|GetActorLocation)) 0.0)
    (Variables|Default|SetObliqueDirection "1.000000,0.000000,0.000000")
    (else
      (Variables|Default|SetObliqueDirection "-1.000000,0.000000,0.000000"))))

(event Collision|EventActorBeginOverlap
  (params (OtherActor :type Actor%20Object%20Reference))
  (|CallParentFunction OtherActor) ; This node is disabled and will not be called.\nDrag off pins to build functionality.
)

(event EventTick
  (params (DeltaSeconds :type Float%20%28single-precision%29))
  (bind _returnvalue (Transformation|GetActorLocation))
  (|CallParentFunction DeltaSeconds)
  (Transformation|SetActorLocation (Math|Vector|MakeVector (+ (.x (Transformation|GetActorLocation)) (* (.x (Variables|Default|GetObliqueDirection)) (Variables|/Game/SpaceShooter/Blueprints/MovementComponent/BP_MovementComponent.BP_MovementComponent_C|GetSpeed (Variables|Default|GetBP_MovementComponent)) DeltaSeconds)) (.y _returnvalue) (.z _returnvalue)) false false))

(fn ConstructionScript
  (|CallParentFunction))