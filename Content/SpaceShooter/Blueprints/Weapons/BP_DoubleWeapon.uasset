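; Space shooter weapon Blueprint that fires two projectiles at once.
; Its Fire override calls the parent, then, if firing is allowed, clears the fire flag and starts a one-shot cooldown timer.
; It spawns the Projectile class at the Muzzle1 and Muzzle2 transforms.
; Each valid projectile receives the weapon's first actor tag.
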(event EventBeginPlay
  (|CallParentFunction) ; This node is disabled and will not be called.\nDrag off pins to build functionality.
)

(fn ConstructionScript
  (|CallParentFunction))

(fn Fire
  (bind _projectile (Variables|Default|GetProjectile))
  (|CallParentFunction)
  (if (Variables|Default|GetCanFireProjectile)
    (Utilities|Time|SetTimerbyEvent (EventDispatchers|CreateEvent :!event EventFireProjectileCooldownFinished) (Variables|Default|GetFireProjectileCooldown))
    (Variables|Default|SetCanFireProjectile false)
    (if (Utilities|IsValidClass _projectile)
      (Utilities|FlowControl|Sequence
        (:then_0
          (bind _returnvalue (Game|SpawnActorfromClass _projectile (Transformation|GetWorldTransform (Variables|Default|GetMuzzle1)) "Undefined" "MultiplyWithRoot" 0 0))
          (Utilities|IsValid _returnvalue
            (:Is%20Valid
              (Utilities|Array|Add (Variables|/Script/Engine.Actor|GetTags _returnvalue) (Utilities|Array|Get(acopy) (Variables|Default|GetTags))))))
        (:then_1
          (bind _returnvalue_2 (Game|SpawnActorfromClass _projectile (Transformation|GetWorldTransform (Variables|Default|GetMuzzle2)) "Undefined" "MultiplyWithRoot" 0 0))
          (Utilities|IsValid _returnvalue_2
            (:Is%20Valid
              (Utilities|Array|Add (Variables|/Script/Engine.Actor|GetTags _returnvalue_2) (Utilities|Array|Get(acopy) (Variables|Default|GetTags))))))))))