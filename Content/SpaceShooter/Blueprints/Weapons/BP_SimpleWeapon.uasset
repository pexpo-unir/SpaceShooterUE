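; BP_SimpleWeapon is a space shooter weapon that fires one projectile per shot, limited by a cooldown.
; Its Fire override calls the parent, then, if firing is allowed, clears CanFireProjectile and starts a one-shot cooldown timer.
; It spawns the Projectile class at the Muzzle transform and copies the weapon's first tag onto the spawned actor.
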(event EventBeginPlay
  (|CallParentFunction) ; This node is disabled and will not be called.\nDrag off pins to build functionality.
)

(fn ConstructionScript
  (|CallParentFunction))

(fn Fire
  (bind _projectile (Variables|Default|GetProjectile))
  (|CallParentFunction)
  (if (Variables|Default|GetCanFireProjectile)
    (Utilities|Time|SetTimerbyEvent (EventDispatchers|CreateEvent :!event EventFireProjectileCooldownFinished) (Variables|Default|GetFireProjectileCooldown))
    (Variables|Default|SetCanFireProjectile false)
    (if (Utilities|IsValidClass _projectile)
      (bind _returnvalue (Game|SpawnActorfromClass _projectile (Transformation|GetWorldTransform (Variables|Default|GetMuzzle)) "Undefined" "MultiplyWithRoot" 0 0))
      (Utilities|IsValid _returnvalue
        (:Is%20Valid
          (Utilities|Array|Add (Variables|/Script/Engine.Actor|GetTags _returnvalue) (Utilities|Array|Get(acopy) (Variables|Default|GetTags))))))))