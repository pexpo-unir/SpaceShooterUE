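; BP_Projectile is a space shooter projectile that flies along the constant right vector and damages ship pawns it overlaps.
; BeginPlay sets the direction on its movement component and starts a lifetime timer that destroys it.
; Overlapped ships sharing a tag with the projectile are ignored.
; Otherwise it spawns an explosion at fixed height with 2D sound, sends damage through the IDamageable interface and destroys itself.
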(event Custom|EventLifetimeEnds
  (Actor|DestroyActor))

(event EventBeginPlay
  ;[1 1 1] Movement direction
  (Variables|/Game/SpaceShooter/Blueprints/MovementComponent/BP_MovementComponent.BP_MovementComponent_C|SetDirection (Variables|Default|GetBP_MovementComponent) (Class|KismetMathLibrary|VectorRight))
  ;[1 1 1] Set lifetime event
  (Utilities|Time|SetTimerbyEvent (delegate Custom|EventLifetimeEnds) (Variables|Default|GetLifetime)))

(event Collision|EventActorBeginOverlap
  (params (OtherActor :type Actor%20Object%20Reference))
  (bind _returnvalue (Transformation|GetActorLocation))
  (Utilities|Casting|CastToBP_ShipPawn OtherActor)
  (bind _hasonetag (CallFunction|CheckifContainsatLeastOneTag self OtherActor))
  (if (not _hasonetag)
    (Utilities|FlowControl|Sequence
      (:then_0
        ;[1 1 1] FX
        (Effects|SpawnEmitteratLocation "/Game/StarterContent/Particles/P_Explosion.P_Explosion" (Math|Vector|MakeVector (.x _returnvalue) (.y _returnvalue) 6e+01))
        (Audio|PlaySound2D "/Game/StarterContent/Audio/Explosion01.Explosion01" 0.5 1.0 0.0 0 0 false))
      (:then_1
        ;[1 1 1] Apply Damage
        (if (Utilities|DoesObjectImplementInterface OtherActor "/Game/SpaceShooter/Blueprints/DamageSystem/IDamageable.IDamageable_C")
          (Class|IDamageable|TakeDamage(Message) OtherActor (Variables|Default|GetDamage))))
      (:then_2
        ;[1 1 1] Destroy
        (Actor|DestroyActor)))))

(fn ConstructionScript)